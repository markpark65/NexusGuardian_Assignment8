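; BP_NexusGuardianItem is the Nexus Guardian item Blueprint, handling the show and hide of its overhead widget.
; PlayFadeIn and PlayFadeOut cast the OverHeadWidget component's widget to WBP_OverHeadWidget, play the matching animation, then immediately set render opacity to fully visible or invisible.
; PlayFadeOut sets opacity on the cast result from PlayFadeIn instead of its own.
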(event EventPlayFadeIn
  (bind _aswbp_over_head_widget (Utilities|Casting|CastToWBP_OverHeadWidget (UserInterface|GetUserWidgetObject (Variables|Default|GetOverHeadWidget))))
  (UserInterface|Animation|PlayAnimation _aswbp_over_head_widget (Variables|/Game/Blueprint/WBP_OverHeadWidget.WBP_OverHeadWidget_C|GetFadeIn _aswbp_over_head_widget) 0.0 1 "Forward" 1.0 false)
  (Widget|SetRenderOpacity _aswbp_over_head_widget 1.0))

(event EventPlayFadeOut
  (bind _aswbp_over_head_widget (Utilities|Casting|CastToWBP_OverHeadWidget (UserInterface|GetUserWidgetObject (Variables|Default|GetOverHeadWidget))))
  (UserInterface|Animation|PlayAnimation _aswbp_over_head_widget (Variables|/Game/Blueprint/WBP_OverHeadWidget.WBP_OverHeadWidget_C|GetFadeOut _aswbp_over_head_widget) 0.0 1 "Forward" 1.0 false)
  (Widget|SetRenderOpacity (stale EventPlayFadeIn _aswbp_over_head_widget) 0.0))

(fn ConstructionScript)