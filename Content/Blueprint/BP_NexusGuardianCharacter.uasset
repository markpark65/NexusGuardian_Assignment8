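; Player character Blueprint for Nexus Guardian that owns the player HUD and displays feedback when an item is purchased.
; BeginPlay creates the HUD widget, stores it and adds it to the viewport.
; OnItemPurchased adds a timed icon widget to the HUD's item slot box, then shows a message for the effect type and hides it after a fixed delay.
; The graph handles only UI and applies no gameplay effects.
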(event EventBeginPlay
  (bind _returnvalue (UserInterface|CreateWidget "/Game/Blueprint/WBP_PlayerHUD.WBP_PlayerHUD_C"))
  (bind _output_get (Variables|Default|SetMyHUD _returnvalue))
  (UserInterface|Viewport|AddtoViewport _output_get 0))

(event EventOnItemPurchased
  (params (EffectType :type EItemEffect%20Enum :default "Slowing") (Time :type Float%20%28single-precision%29))
  (bind _myhud (Variables|Default|GetMyHUD))
  (bind _myhud_2 (Variables|Default|GetMyHUD))
  (bind _myhud_3 (Variables|Default|GetMyHUD))
  (bind _itemnametext (Variables|/Game/Blueprint/WBP_PlayerHUD.WBP_PlayerHUD_C|GetItemNameText _myhud_2))
  (bind _itemnametext_2 (Variables|/Game/Blueprint/WBP_PlayerHUD.WBP_PlayerHUD_C|GetItemNameText _myhud))
  (Utilities|FlowControl|Sequence
    (:then_0
      (bind _returnvalue (UserInterface|CreateWidget "/Game/Blueprint/WBP_ItemIcon.WBP_ItemIcon_C" 0 Time Time EffectType))
      (Class|HorizontalBox|AddChildtoHorizontalBox (Variables|/Game/Blueprint/WBP_PlayerHUD.WBP_PlayerHUD_C|GetItemSlotBox (Variables|Default|GetMyHUD)) _returnvalue))
    (:then_1
      (switch Utilities|FlowControl|Switch|SwitchonEItemEffect EffectType
        (:Slowing
          (Rendering|Components|TextRender|SetText (Variables|/Game/Blueprint/WBP_PlayerHUD.WBP_PlayerHUD_C|GetItemNameText _myhud_3) "SPEED DOWN!")
          (Widget|SetVisibility _itemnametext "Visible")
          (Utilities|FlowControl|Delay 5.0)
          (Widget|SetVisibility _itemnametext_2 "Hidden"))
        (:Reverse
          (Rendering|Components|TextRender|SetText (Variables|/Game/Blueprint/WBP_PlayerHUD.WBP_PlayerHUD_C|GetItemNameText _myhud_3) "REVERSE CONTROL!")
          (Widget|SetVisibility _itemnametext "Visible")
          (Utilities|FlowControl|Delay 5.0)
          (Widget|SetVisibility _itemnametext_2 "Hidden"))
        (:Blind
          (Rendering|Components|TextRender|SetText (Variables|/Game/Blueprint/WBP_PlayerHUD.WBP_PlayerHUD_C|GetItemNameText _myhud_3) "BLIND!")
          (Widget|SetVisibility _itemnametext "Visible")
          (Utilities|FlowControl|Delay 5.0)
          (Widget|SetVisibility _itemnametext_2 "Hidden"))
        (:PowerUp
          (Rendering|Components|TextRender|SetText (Variables|/Game/Blueprint/WBP_PlayerHUD.WBP_PlayerHUD_C|GetItemNameText _myhud_3) "POWER UP!")
          (Widget|SetVisibility _itemnametext "Visible")
          (Utilities|FlowControl|Delay 5.0)
          (Widget|SetVisibility _itemnametext_2 "Hidden"))
        (:Heal
          (Rendering|Components|TextRender|SetText (Variables|/Game/Blueprint/WBP_PlayerHUD.WBP_PlayerHUD_C|GetItemNameText _myhud_3) "HEALED!")
          (Widget|SetVisibility _itemnametext "Visible")
          (Utilities|FlowControl|Delay 5.0)
          (Widget|SetVisibility _itemnametext_2 "Hidden"))))))

(fn ConstructionScript)